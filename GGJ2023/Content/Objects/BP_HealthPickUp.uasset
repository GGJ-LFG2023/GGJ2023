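; BP_HealthPickUp is a health pickup for the side-scroller character that spins and bobs in place.
; A self-restarting SpinBob timeline drives a full yaw rotation and a Z offset added to the actor's current location on each update.
; When the player pawn overlaps its sphere, it increments the character's Health if below the cap of three, then destroys itself; at full health it remains.
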(event `self.ReceiveBeginPlay`
  (`self.Spin&BobEvent`))

(event `Spin&BobEvent`
  (bind (_actor_x _actor_y _actor_z) (`self.ActorLocation`))
  (bind (_direction _bob _spin) (`Timeline|Spin&Bob` :!via `PlayFromStart`)
    (:`Update`
      (`self.K2_SetActorLocation` (`KismetMathLibrary.MakeVector` _actor_x _actor_y (+ _actor_z (`KismetMathLibrary.Lerp` -2.0 2.0 _bob))))
      (`self.K2_SetActorRotation` (`KismetMathLibrary.MakeRotator` 0.0 0.0 (`KismetMathLibrary.Lerp` 0.0 360.0 _spin))))
    (:`Finished`
      (`self.Spin&BobEvent`))))

(event `self.Sphere.OnComponentBeginOverlap`
  (params (OverlappedComponent :type "PrimitiveComponent Object Reference") (OtherActor :type "Actor Object Reference") (OtherComp :type "PrimitiveComponent Object Reference") (OtherBodyIndex :type Integer) (bFromSweep :type Boolean) (SweepResult :type "HitResult Structure (by ref)"))
  (bind _returnvalue (`GameplayStatics.GetPlayerPawn` 0))
  (if (== OtherActor _returnvalue)
    (bind _asside_scroller_character (cast `/Game/SideScrollerBP/Blueprints/SideScrollerCharacter` _returnvalue))
    (bind _health (`/Game/SideScrollerBP/Blueprints/SideScrollerCharacter.health` _asside_scroller_character))
    (if (not (>= _health 3.0))
      (`/Engine/EditorBlueprintResources/StandardMacros.IncrementFloat` _health
        (:`  `
          (`self.K2_DestroyActor`))))))

(fn `ActorLocation`
  (returns (`Actor X` :type "Float (double-precision)") (`Actor Y` :type "Float (double-precision)") (`Actor Z` :type "Float (double-precision)"))
  (bind (_returnvalue_x _returnvalue_y _returnvalue_z) (`KismetMathLibrary.BreakVector` (`self.K2_GetActorLocation`)))
  (return _returnvalue_x _returnvalue_y _returnvalue_z))

(fn `UserConstructionScript`)