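; BP_ZipLine is a zip line object whose platform travels from a start point to an end point once the player enters its trigger box.
; The overlap waits briefly, then plays the Zip timeline, which lerps the platform's world location between the two points.
; It also binds to the player pawn's destroyed event to snap the platform back to the start.
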(event `StartMoving`
  (bind (_direction _move) (`Timeline|Zip`)
    (:`Update`
      (`SceneComponent.K2_SetWorldLocation` (`self.PlatformBase`) (`KismetMathLibrary.VLerp` (`SceneComponent.K2_GetComponentLocation` (`self.StartPoint`)) (`SceneComponent.K2_GetComponentLocation` (`self.EndPoint`)) _move) false false))))

(event `self.Box.OnComponentBeginOverlap`
  (params (OverlappedComponent :type "PrimitiveComponent Object Reference") (OtherActor :type "Actor Object Reference") (OtherComp :type "PrimitiveComponent Object Reference") (OtherBodyIndex :type Integer) (bFromSweep :type Boolean) (SweepResult :type "HitResult Structure (by ref)"))
  (bind _returnvalue (`GameplayStatics.GetPlayerPawn` 0))
  (if (== OtherActor _returnvalue)
    (add `self.OnDestroyed` _returnvalue (delegate `ResetZipLine`))
    (`KismetSystemLibrary.Delay` 2.0)
    (`self.StartMoving`)))

(event `ResetZipLine` :!signature `self.OnDestroyed`
  (params (DestroyedActor :type "Actor Object Reference"))
  (`SceneComponent.K2_SetWorldLocation` (`self.PlatformBase`) (`SceneComponent.K2_GetComponentLocation` (`self.StartPoint`)) false false))

(fn `UserConstructionScript`)