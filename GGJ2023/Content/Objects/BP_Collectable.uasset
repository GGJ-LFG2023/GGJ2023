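; BP_Collectable is a seed pickup that spins and shrinks away when something overlaps its collision sphere.
; On BeginPlay, the Spin timeline adds to the actor's yaw each update and restarts in reverse from the end when finished.
; Any sphere overlap, without a player check, plays the Shrink timeline, which adds to Y and Z scale, leaving X unchanged, and destroys the actor once both are zero or below.
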(event `self.ReceiveBeginPlay`
  (bind (_returnvalue_roll _returnvalue_pitch _returnvalue_yaw) (`KismetMathLibrary.BreakRotator` (`self.K2_GetActorRotation`)))
  ;[1 1 1] Code for Seed to rotate
  (bind (_direction _zrotation) (`Timeline|Spin` :!label _label)
    (:`Update`
      (`self.K2_SetActorRotation` (`KismetMathLibrary.MakeRotator` _returnvalue_roll _returnvalue_pitch (+ _zrotation _returnvalue_yaw))))
    (:`Finished`
      (goto _label :!via `ReverseFromEnd`))))

(event `self.SphereCollision.OnComponentBeginOverlap`
  (params (OverlappedComponent :type "PrimitiveComponent Object Reference") (OtherActor :type "Actor Object Reference") (OtherComp :type "PrimitiveComponent Object Reference") (OtherBodyIndex :type Integer) (bFromSweep :type Boolean) (SweepResult :type "HitResult Structure (by ref)"))
  (bind (_returnvalue_x _returnvalue_y _returnvalue_z) (`KismetMathLibrary.BreakVector` (`self.GetActorScale3D`)))
  ;[1 1 1] Collosion Code with Seed (Where Player actor collides with seed)
  (bind (_direction _shrinkz _shrinky) (`Timeline|Shrink`)
    (:`Update`
      (if (and (<= _returnvalue_y 0.0) (<= _returnvalue_z 0.0))
        (`self.K2_DestroyActor`)
        (else
          (`self.SetActorScale3D` (`KismetMathLibrary.MakeVector` _returnvalue_x (+ _shrinky _returnvalue_y) (+ _shrinkz _returnvalue_z))))))))

(fn `UserConstructionScript`)