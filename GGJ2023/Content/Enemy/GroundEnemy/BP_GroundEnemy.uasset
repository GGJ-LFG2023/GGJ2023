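; BP_GroundEnemy is a ground enemy that patrols, chases the player and damages them on contact.
; Patrol loops AI MoveTo between two target points with short pauses, starting on BeginPlay.
; The NoticePlayer overlap switches movement to chasing the player, and leaving it resumes patrol after a brief delay.
; HurtPlayer overlap decrements Health on BP_SideScrollerCharacter once per entry, and its trailing Delay leads to nothing.
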(event `self.ReceiveBeginPlay`
  (`self.Patrol`))

(event `Patrol`
  (`|AIMoveTo` self (0.0 0.0 0.0) (`self.TargetPoint1`)
    (:`OnSuccess`
      (`KismetSystemLibrary.Delay` 0.25)
      (`|AIMoveTo` self (0.0 0.0 0.0) (`self.TargetPoint2`)
        (:`OnSuccess`
          (`KismetSystemLibrary.Delay` 0.25)
          (`self.Patrol`))))))

(event `self.Notice Player.OnComponentBeginOverlap`
  (params (OverlappedComponent :type "PrimitiveComponent Object Reference") (OtherActor :type "Actor Object Reference") (OtherComp :type "PrimitiveComponent Object Reference") (OtherBodyIndex :type Integer) (bFromSweep :type Boolean) (SweepResult :type "HitResult Structure (by ref)"))
  (bind _returnvalue (`GameplayStatics.GetPlayerPawn` 0))
  (if (== OtherActor _returnvalue)
    (`|AIMoveTo` self (0.0 0.0 0.0) _returnvalue)))

(event `self.Notice Player.OnComponentEndOverlap`
  (params (OverlappedComponent :type "PrimitiveComponent Object Reference") (OtherActor :type "Actor Object Reference") (OtherComp :type "PrimitiveComponent Object Reference") (OtherBodyIndex :type Integer))
  (if (== OtherActor (`GameplayStatics.GetPlayerPawn` 0))
    (`KismetSystemLibrary.Delay` 0.5)
    (`self.Patrol`)))

(event `self.HurtPlayer.OnComponentBeginOverlap`
  (params (OverlappedComponent :type "PrimitiveComponent Object Reference") (OtherActor :type "Actor Object Reference") (OtherComp :type "PrimitiveComponent Object Reference") (OtherBodyIndex :type Integer) (bFromSweep :type Boolean) (SweepResult :type "HitResult Structure (by ref)"))
  (bind _returnvalue (`GameplayStatics.GetPlayerPawn` 0))
  (if (== OtherActor _returnvalue)
    (bind _asbp_side_scroller_character (cast `/Game/GrapplingSideScrollerCharacter/BP_SideScrollerCharacter` _returnvalue))
    (`/Engine/EditorBlueprintResources/StandardMacros.DecrementFloat` (`/Game/GrapplingSideScrollerCharacter/BP_SideScrollerCharacter.health` _asbp_side_scroller_character)
      (:`  `
        (`KismetSystemLibrary.Delay` 1.5)))))

(fn `UserConstructionScript`)