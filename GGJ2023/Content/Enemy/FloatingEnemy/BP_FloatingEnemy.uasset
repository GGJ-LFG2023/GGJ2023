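; Floating enemy for the side-scroller that patrols between two placed patrol points and damages the player on contact.
; A timeline lerps its location between the points and adds a vertical bob, with a FlipFlop alternating reverse and play at each end.
; Player overlap with its sphere decrements the character's Health; the trailing Delay drives nothing.
; FlipPatrolDestination is an unfinished, uncalled stub.
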(event `self.ReceiveBeginPlay`
  (`self.Patrol`))

(event `self.ReceiveActorBeginOverlap`
  (params (OtherActor :type "Actor Object Reference")))

(event `self.ReceiveTick`
  (params (DeltaSeconds :type "Float (single-precision)")))

(event `Patrol`
  (bind (_direction _movetopoint _bob) (`Timeline|PartolTimeLine` :!via `PlayFromStart` :!label _label)
    (:`Update`
      (bind (_returnvalue_x _returnvalue_y _returnvalue_z) (`KismetMathLibrary.BreakVector` (`KismetMathLibrary.VLerp` (`self.PatrolPoint1Location`) (`self.PatrolPoint2Location`) _movetopoint)))
      (`self.K2_SetActorLocation` (`KismetMathLibrary.MakeVector` _returnvalue_x _returnvalue_y (+ _returnvalue_z (`KismetMathLibrary.Lerp` -20.0 20.0 _bob)))))
    (:`Finished`
      (`self.ContinuePatrol`))))

(event `ContinuePatrol`
  (`/Engine/EditorBlueprintResources/StandardMacros.FlipFlop`
    (:`A`
      (goto _label :!via `Reverse`))
    (:`B`
      (goto _label))))

(event `self.Sphere.OnComponentBeginOverlap`
  (params (OverlappedComponent :type "PrimitiveComponent Object Reference") (OtherActor :type "Actor Object Reference") (OtherComp :type "PrimitiveComponent Object Reference") (OtherBodyIndex :type Integer) (bFromSweep :type Boolean) (SweepResult :type "HitResult Structure (by ref)"))
  (if (== OtherActor (`GameplayStatics.GetPlayerPawn` 0))
    (`self.Get Player`)
    (`/Engine/EditorBlueprintResources/StandardMacros.DecrementFloat` (`/Game/GrapplingSideScrollerCharacter/BP_SideScrollerCharacter.health` (`self.PlayerChar`))
      (:`  `
        (`KismetSystemLibrary.Delay` 1.5)))))

(fn `FlipPatrolDestination`
  (bind _returnvalue (`SceneComponent.K2_GetComponentLocation` (`self.DefaultSceneRoot`)))
  (if (== (`self.PatrolPoint1Location`) _returnvalue :`ErrorTolerance` 0.01)
    _
    (elif (== (`self.PatrolPoint2Location`) _returnvalue :`ErrorTolerance` 0.01)
      _)))

(fn `Get Player`
  (bind _asbp_side_scroller_character (cast `/Game/GrapplingSideScrollerCharacter/BP_SideScrollerCharacter` (`GameplayStatics.GetPlayerPawn` 0)))
  (set `self.PlayerChar` _asbp_side_scroller_character))

(fn `PatrolPoint1Location`
  (returns (WorldLocation :type "Vector Structure"))
  (return (`SceneComponent.K2_GetComponentLocation` (`/Game/Enemy/FloatingEnemy/BP_PartolPoint.DefaultSceneRoot` (`self.PartolPoint1`)))))

(fn `PatrolPoint2Location`
  (returns (WorldLocation :type "Vector Structure"))
  (return (`SceneComponent.K2_GetComponentLocation` (`/Game/Enemy/FloatingEnemy/BP_PartolPoint.DefaultSceneRoot` (`self.PartolPoint2`)))))

(fn `UserConstructionScript`)